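; BP_PlayV2 is a player Blueprint that assembles its body from modular skeletal mesh parts.
; The construction script sets Mesh as leader pose component for HeadMesh, LegMesh, SkeletalMesh and SkeletalMesh1, so the parts follow one animated skeleton.
; The event graph holds only disabled placeholder events, so the graphs add no gameplay logic.
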(fn `UserConstructionScript`
  (bind _mesh (`self.Mesh`))
  (`SkinnedMeshComponent.SetLeaderPoseComponent` (`self.HeadMesh`) _mesh true false)
  (`SkinnedMeshComponent.SetLeaderPoseComponent` (`self.LegMesh`) _mesh true false)
  (`SkinnedMeshComponent.SetLeaderPoseComponent` (`self.SkeletalMesh`) (`self.Mesh`) true false)
  (`SkinnedMeshComponent.SetLeaderPoseComponent` (`self.SkeletalMesh1`) (`self.Mesh`) true false))